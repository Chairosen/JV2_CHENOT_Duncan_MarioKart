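; Item manager component for a vehicle game, owned by the player controller, that holds the player's current item.
; GetItem always grants the shell item, and SetItem stores the item and fires an item-change notification.
; UseItem launches the held item, passing in the owning controller, then clears the slot.
; Tick prints the held item's name each frame as debug output.
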(event EventTick
  (params (DeltaSeconds :type Float%20%28single-precision%29))
  (bind _currentitem (Variables|Default|GetcurrentItem)
    (:then
      (Development|PrintString (Utilities|GetDisplayName _currentitem)))
    (:else)))

(fn GetItem
  (CallFunction|SetItem "/Game/Data/Items/ID_S_Shell.ID_S_Shell"))

(fn SetItem
  (params (currentItem :type BP%20Item%20Data%20Object%20Reference))
  (bind _output_get (Variables|Default|SetcurrentItem currentItem))
  (Default|CallOnItemChange _output_get))

(fn UseItem
  (bind _currentitem (Variables|Default|GetcurrentItem)
    (:then
      (Default|LaunchItem _currentitem (.AsBP%20Vehicle%20Adv%20Player%20Controller (Utilities|Casting|CastToBP_VehicleAdvPlayerController (Components|GetOwner))))
      (CallFunction|SetItem))
    (:else)))