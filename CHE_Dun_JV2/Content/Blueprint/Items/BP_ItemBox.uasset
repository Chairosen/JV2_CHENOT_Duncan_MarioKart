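; BP_ItemBox is a pickup box that grants an item to a vehicle that drives into it.
; When the Cube overlaps a BP_VehicleAdvPawnBase, it calls GetItem on that pawn's controller, leaving the item logic to the controller.
; It then hides the Cube and disables its collision, restoring visibility and query-only collision after a brief delay so the box is reusable.
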(event OnComponentBeginOverlap(Cube)
  (params (OverlappedComponent :type Primitive%20Component%20Object%20Reference) (OtherActor :type Actor%20Object%20Reference) (OtherComp :type Primitive%20Component%20Object%20Reference) (OtherBodyIndex :type Integer) (bFromSweep :type Boolean) (SweepResult :type Hit%20Result%20Structure%20%28by%20ref%29))
  (bind _asbp_vehicle_adv_pawn_base (Utilities|Casting|CastToBP_VehicleAdvPawnBase OtherActor))
  (bind _asbp_vehicle_adv_player_controller (Default|GetCastedController _asbp_vehicle_adv_pawn_base))
  (Default|GetItem _asbp_vehicle_adv_player_controller)
  (CallFunction|Disapear))

(event Custom|Disapear
  (bind _cube (Variables|Default|GetCube))
  (bind _cube_2 (Variables|Default|GetCube))
  (Rendering|SetVisibility _cube_2 false false)
  (Collision|SetCollisionEnabled _cube_2 "NoCollision")
  (Utilities|FlowControl|Delay 0.2)
  (Rendering|SetVisibility _cube true false)
  (Collision|SetCollisionEnabled _cube "QueryOnly"))

(fn ConstructionScript)