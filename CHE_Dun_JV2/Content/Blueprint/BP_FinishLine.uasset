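; Finish line trigger for a vehicle game that counts turns, apparently laps.
; OnTrigger calls AddTurn on the player controller's BP_AC_TurnManager component, then refreshes the UI.
; A separate Deactivate volume switches off the Box's overlap events while a vehicle pawn is inside, restoring them shortly after it leaves, which likely blocks counting from that side.
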(event OnComponentBeginOverlap(Deactivate)
  (params (OverlappedComponent :type Primitive%20Component%20Object%20Reference) (OtherActor :type Actor%20Object%20Reference) (OtherComp :type Primitive%20Component%20Object%20Reference) (OtherBodyIndex :type Integer) (bFromSweep :type Boolean) (SweepResult :type Hit%20Result%20Structure%20%28by%20ref%29))
  (Utilities|Casting|CastToBP_VehicleAdvPawnBase OtherActor)
  (Variables|/Script/Engine.PrimitiveComponent|SetbGenerateOverlapEvents (Variables|Default|GetBox) false))

(event OnComponentEndOverlap(Deactivate)
  (params (OverlappedComponent :type Primitive%20Component%20Object%20Reference) (OtherActor :type Actor%20Object%20Reference) (OtherComp :type Primitive%20Component%20Object%20Reference) (OtherBodyIndex :type Integer))
  (Utilities|Casting|CastToBP_VehicleAdvPawnBase OtherActor)
  (Utilities|FlowControl|Delay 0.2)
  (Variables|/Script/Engine.PrimitiveComponent|SetbGenerateOverlapEvents (Variables|Default|GetBox) true))

(event EventOnTrigger
  (bind _controller (CallFunction|GetPlayerController))
  (Default|AddTurn (Actor|GetComponentbyClass _controller "/Game/Blueprint/BP_AC_TurnManager.BP_AC_TurnManager_C"))
  (Default|UpdateUI _controller))

(fn ConstructionScript
  (|CallParentFunction))